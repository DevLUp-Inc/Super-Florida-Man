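; Balloon actor that pushes its static mesh upward with a constant physics force every tick.
; The construction script creates a dynamic instance of M_Base_Balloon and gives it a fully saturated, full-brightness random hue.
; The random stream is seeded from the truncated world X position, so the color is repeatable per placement, and balloons at the same X share a color.
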(event `self.ReceiveTick`
  (params (DeltaSeconds :type "Float (single-precision)"))
  (`PrimitiveComponent.AddForce` (`self.StaticMesh`) (0.0 0.0 100.0) "None" false))

(fn `UserConstructionScript`
  (bind _returnvalue (`KismetMaterialLibrary.CreateDynamicMaterialInstance` "/Game/Assets/Models/Balloon/M_Base_Balloon.M_Base_Balloon"))
  (`MaterialInstanceDynamic.SetVectorParameterValue` _returnvalue "Base Color" (`KismetMathLibrary.HSVToRGB` (`KismetMathLibrary.RandomFloatInRangeFromStream` 0.0 360.0 (`KismetMathLibrary.MakeRandomStream` (`KismetMathLibrary.FTrunc` (.x (`self.K2_GetActorLocation`))))) 1.0 1.0))
  (`PrimitiveComponent.SetMaterial` (`self.StaticMesh`) 0 _returnvalue))
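; Water plane Blueprint that tiles a static mesh into a grid, sized by RepeatX and RepeatY.
; The construction script runs nested loops over both counts, adding a mesh component every 1000 units along local X and Y.
; A NAND check skips only the origin cell.
; The event graph holds only disabled placeholder events, so there is no runtime logic.
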(fn `UserConstructionScript`
  (for _index (range (+ (`self.repeat X`) 1))
    (for _index_2 (range (+ (`self.repeat Y`) 1))
      (if (`KismetMathLibrary.BooleanNAND` (== _index 0) (== _index_2 0))
        (`AddComponent|NODE_AddStaticMeshComponent-0` :`RelativeTransform` (`KismetMathLibrary.MakeTransform` (`KismetMathLibrary.MakeVector` (* _index 1000.0) (* _index_2 1000.0))))))))
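; Player character pawn that moves by physics forces on its capsule, with mouse look, double jump and an orange pickup counter.
; Walk axes push along the Cube's facing, MouseX yaws the Cube and MouseY pitches the spring arm.
; Jump uses a downward ground trace to refill two jumps, while Tick applies constant downward acceleration.
; IncrementOrangeCount raises the orange tally and prints a message.
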(event `InputAction|Jump`
  (params (Key :type "Key Structure"))
  (bind _returnvalue (`SceneComponent.K2_GetComponentLocation` (`self.Capsule`)))
  (:`Pressed`
    (bind (_outhit _returnvalue_2) (`KismetSystemLibrary.LineTraceSingle` :`Start` _returnvalue :`End` (- _returnvalue (0.0 0.0 100.0)) :`TraceChannel` "TraceTypeQuery1" :`DrawDebugType` "Persistent"))
    (if _returnvalue_2
      (set `self.jumpCount` 2)
      (`PrimitiveComponent.AddForce` (`self.Capsule`) (0.0 0.0 50000.0) "None" false :!label _label)
      (`/Engine/EditorBlueprintResources/StandardMacros.DecrementInt` (`self.jumpCount`))
      (elif (> (`self.jumpCount`) 0)
        (goto _label)))))

(event `InputAxis|walkForward`
  (params (AxisValue :type "Float (single-precision)"))
  (`PrimitiveComponent.AddForce` (`self.Capsule`) (* (* (`SceneComponent.GetForwardVector` (`self.Cube`)) AxisValue) 2000.0) "None" false))

(event `InputAxis|walkRight`
  (params (AxisValue :type "Float (single-precision)"))
  (`PrimitiveComponent.AddForce` (`self.Capsule`) (* (* (`SceneComponent.GetRightVector` (`self.Cube`)) AxisValue) 2000.0) "None" false))

(event `InputAxis|MouseX`
  (params (AxisValue :type "Float (single-precision)"))
  (`SceneComponent.K2_AddLocalRotation` (`self.Cube`) (`KismetMathLibrary.MakeRotator` 0.0 0.0 AxisValue) false false))

(event `self.ReceiveTick`
  (params (DeltaSeconds :type "Float (single-precision)"))
  (`PrimitiveComponent.AddForce` (`self.Capsule`) (0.0 0.0 -1000.0) "None" true))

(event `InputAxis|MouseY`
  (params (AxisValue :type "Float (single-precision)"))
  (`SceneComponent.K2_AddLocalRotation` (`self.SpringArm`) (`KismetMathLibrary.MakeRotator` 0.0 AxisValue) false false))

(fn `IncrementOrangeCount`
  (`/Engine/EditorBlueprintResources/StandardMacros.IncrementInt` (`self.Oranges`)
    (:`  `
      (`KismetSystemLibrary.PrintString` "You Have More Orange"))))

(fn `UserConstructionScript`)